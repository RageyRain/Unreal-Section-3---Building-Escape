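; Staircase prop that rises once from its placed position when the RaiseStairs OnRaise event fires.
; A DoOnce gate spawns a steam particle effect at the SmokeLocation actor and plays the StairRaise timeline.
; The timeline's RaisePosition offset is added to the location cached at BeginPlay to move the static mesh.
; The OnLower event is empty, so the stairs never descend.
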(event OnRaise(RaiseStairs)
  (Utilities|FlowControl|DoOnce false
    (:Completed
      (Effects|SpawnEmitteratLocation "/Game/Particles/P_Steam_Lit.P_Steam_Lit" (Transformation|GetActorLocation (Variables|Default|GetSmokeLocation)))
      (bind _raise_position (Timeline|Stair%20Raise Play)
        (:Update
          (Transformation|SetWorldLocation (Variables|Debug|GetStaticMeshComponent) (+ _raise_position (Variables|Default|GetInitialLocation)) false false))))))

(event OnLower(RaiseStairs))

(event EventBeginPlay
  (Variables|Default|SetInitialLocation (Transformation|GetActorLocation)))

(fn ConstructionScript)